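; BP_Player is a rolling-ball player character that moves by applying torque to its Sphere component.
; Each tick, Movement scales the left/right and forward/backward axis inputs by MoveMultiplier and applies them as mass-independent angular acceleration.
; Holding Left Shift routes those values through BoostsSpeedValues, which multiplies them by Boost.
; On BeginPlay, the camera fades in from fully faded to open the level.
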(event `self.ReceiveBeginPlay`
  (`self.Level Start Camera Fade` 3.0))

(event `self.ReceiveTick`
  (params (DeltaSeconds :type "Float (single-precision)"))
  (`self.Movement` (`self.Boost is Activated?`)))

(event `Key|LeftShift`
  (params (Key :type "Key Structure"))
  (:`Pressed`
    (set `self.Boost is Activated?` true))
  (:`Released`
    (set `self.Boost is Activated?` false)))

(fn `Level Start Camera Fade`
  (params (`Fade Duration` :type "Float (double-precision)" :default 3.0))
  (`PlayerCameraManager.StartCameraFade` :`self` (`GameplayStatics.GetPlayerCameraManager` 0) :`FromAlpha` 1.0 :`Duration` `Fade Duration`))

(fn `Movement`
  (params (Boost :type Boolean))
  (bind (_left___right _forward___backwards) (`self.Torque Calculation`))
  (if Boost
    (bind (_left___right_2 _forward___backward) (`self.Boosts Speed Values` _left___right _forward___backwards)
      (:`Exec`
        (`PrimitiveComponent.AddTorqueInRadians` (`self.Sphere`) (`KismetMathLibrary.MakeVector` _left___right_2 _forward___backward) "None" true)))
    (else
      (`PrimitiveComponent.AddTorqueInRadians` (`self.Sphere`) (`KismetMathLibrary.MakeVector` _left___right _forward___backwards) "None" true))))

(fn `Torque Calculation`
  (returns (`Left / Right` :type "Float (double-precision)") (`Forward / Backwards` :type "Float (double-precision)"))
  (bind _movemultiplier (`self.MoveMultiplier`))
  (return (* (`self.GetInputAxisValue`) _movemultiplier) (* _movemultiplier (`self.GetInputAxisValue`))))

(fn `UserConstructionScript`)