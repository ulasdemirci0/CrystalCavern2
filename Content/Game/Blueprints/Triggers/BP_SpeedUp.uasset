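; BP_SpeedUp is a trigger that changes the player ball's move multiplier when the player pawn overlaps it.
; On begin overlap it saves the current MoveMultiplier, optionally brakes, then applies the SpeedUp value.
; A positive ReturnBackupSpeedDelay restores the saved multiplier after that delay; otherwise the change persists.
; Optional brakes on entry and exit overwrite the linear and angular physics velocities of the player's Sphere.
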(event `self.CollisionComponent.OnComponentBeginOverlap`
  (params (OverlappedComponent :type "PrimitiveComponent Object Reference") (OtherActor :type "Actor Object Reference") (OtherComp :type "PrimitiveComponent Object Reference") (OtherBodyIndex :type Integer) (bFromSweep :type Boolean) (SweepResult :type "HitResult Structure (by ref)"))
  ;[1 1 1] Begin Overlap
  (`self.Is Player` OtherActor
    (:`Is Player`
      (`self.Cast BP Player`
        (:`Cast Success`
          (`self.Create Backup Speed`)
          (if (`self.Brake Begin`)
            (`self.Brake Now`))
          (`self.Change Player Move Multiplier`)
          (`self.Return Backup Speed Then Delay`))))))

(event `self.CollisionComponent.OnComponentEndOverlap`
  (params (OverlappedComponent :type "PrimitiveComponent Object Reference") (OtherActor :type "Actor Object Reference") (OtherComp :type "PrimitiveComponent Object Reference") (OtherBodyIndex :type Integer))
  ;[1 1 1] Brake End Overlap
  (`self.Is Player` OtherActor
    (:`Is Player`
      (`self.Cast BP Player`
        (:`Cast Success`
          (if (`self.Brake End`)
            (`self.Brake Now`)))))))

(fn `Brake Now`
  (bind _sphere (`/Game/Game/Blueprints/BP_Player.Sphere` (`self.BP_Player`)))
  (`PrimitiveComponent.SetAllPhysicsLinearVelocity` _sphere (0.0 0.0 0.0) false)
  (`PrimitiveComponent.SetAllPhysicsAngularVelocityInRadians` _sphere (0.0 0.0 0.0) false))

(fn `Change Player Move Multiplier`
  (set `/Game/Game/Blueprints/BP_Player.MoveMultiplier` (`self.SpeedUp`) (`self.BP_Player`)))

(fn `Create Backup Speed`
  (set `self.BackUp` (`/Game/Game/Blueprints/BP_Player.MoveMultiplier` (`self.BP_Player`))))

(fn `UserConstructionScript`)