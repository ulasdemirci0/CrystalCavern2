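; BP_Crystal_Blue is a collectible crystal that flies into the player and vanishes when the player pawn overlaps its sphere.
; On overlap it stores its location, scale and point light intensity, then plays the BlendLerp timeline.
; Three timeline tracks lerp the crystal toward the player's live location, shrink it to zero and fade its light.
; The actor destroys itself when the timeline finishes, with no score or inventory update.
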(event `self.Sphere.OnComponentBeginOverlap`
  (params (OverlappedComponent :type "PrimitiveComponent Object Reference") (OtherActor :type "Actor Object Reference") (OtherComp :type "PrimitiveComponent Object Reference") (OtherBodyIndex :type Integer) (bFromSweep :type Boolean) (SweepResult :type "HitResult Structure (by ref)"))
  (`self.Is Player?` OtherActor
    (:`Is Player`
      (`self.Store Start Values`)
      (bind (_direction _collection_progress _scaling_progress _light_progress) (`Timeline|Blend Lerp`)
        (:`Update`
          (`self.Move to Player` _collection_progress)
          (`self.Scale Crystal` _scaling_progress)
          (`self.Adjust Light` _light_progress))
        (:`Finished`
          (`self.K2_DestroyActor`))))))

(fn `Adjust Light`
  (params (`Light Progress` :type "Float (double-precision)"))
  (`LightComponent.SetIntensity` (`self.PointLight`) (`KismetMathLibrary.Lerp` (`self.Light Intensity`) 0.0 `Light Progress`)))

(fn `Move to Player`
  (params (`Collection Progress` :type "Float (double-precision)"))
  (`self.K2_SetActorLocation` (`KismetMathLibrary.VLerp` (`self.Start Location`) (`self.K2_GetActorLocation` (`GameplayStatics.GetPlayerPawn` 0)) `Collection Progress`)))

(fn `Scale Crystal`
  (params (`Scaling Progress` :type "Float (double-precision)"))
  (`self.SetActorScale3D` (`KismetMathLibrary.VLerp` (`self.Start Scale`) (0.0 0.0 0.0) `Scaling Progress`)))

(fn `Store Start Values`
  (set `self.Light Intensity` (`LightComponentBase.Intensity` (`self.PointLight`)))
  (set `self.Start Location` (`self.K2_GetActorLocation`))
  (set `self.Start Scale` (`self.GetActorScale3D`)))

(fn `UserConstructionScript`)