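; BP_Player is a player Blueprint that rolls a physics sphere from movement input.
; Each tick it scales the left/right and forward/backward axis values by a move multiplier and applies them to the Sphere as torque in acceleration-change mode, so mass is ignored.
; On BeginPlay it calls StartFade, which fades the player camera in from fully faded.
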(event `self.ReceiveBeginPlay`
  (`|ExecutionSequence`
    (:`then_0`
      (`PlayerCameraManager.StartCameraFade` :`self` (`GameplayStatics.GetPlayerCameraManager` 0) :`FromAlpha` 1.0 :`ToAlpha` 0.0 :`Duration` 5.0))))

(event `self.ReceiveTick`
  (params (DeltaSeconds :type "Float (single-precision)"))
  (bind _movemultiplier (`self.MoveMultiplier`))
  (`PrimitiveComponent.AddTorqueInRadians` (`self.Sphere`) (`KismetMathLibrary.MakeVector` (* _movemultiplier (`self.GetInputAxisValue`)) (* (`self.GetInputAxisValue`) _movemultiplier)) "None" true))

(fn `UserConstructionScript`)